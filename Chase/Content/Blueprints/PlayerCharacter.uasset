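; Player character Blueprint for a chase game, handling the game UI, mouse cursor and status particle effects.
; On begin play it switches off both particle systems, adds the GameUI widget to the viewport and shows the cursor.
; A game state change to Setup in ChaseGameState hides the cursor.
; Tick polls Invulnerable and ChargeTimer to toggle the invulnerability and fire particles, with neither variable set in this graph.
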(event `self.ReceiveBeginPlay`
  (bind _returnvalue (`GameplayStatics.GetPlayerController` null))
  (`ActorComponent.Deactivate` (`self.FireParticles`))
  (`ActorComponent.Deactivate` (`self.InvulnerableParticles`))
  (bind _returnvalue_2 (`|CreateWidget` "/Game/Blueprints/UMG/GameUI.GameUI_C" _returnvalue))
  (`UserWidget.AddToViewport` _returnvalue_2)
  (set `PlayerController.bShowMouseCursor` true _returnvalue))

(event `self.GameStateChanged`
  (bind _aschase_game_state (cast `ChaseGameState` (`GameplayStatics.GetGameState` null)))
  (switch `ChaseGameState.EChaseGameState` (`ChaseGameState.CurrentGameState` _aschase_game_state)
    (:`Setup`
      (set `PlayerController.bShowMouseCursor` false (`GameplayStatics.GetPlayerController` null)))))

(event `self.ReceiveTick`
  (params (DeltaSeconds :type "Float (single-precision)"))
  (bind _fireparticles (`self.FireParticles`))
  (bind _invulnerableparticles (`self.InvulnerableParticles`))
  (if (`self.Invulnerable`)
    (`ActorComponent.Activate` _invulnerableparticles false)
    (else
      (`ActorComponent.Deactivate` _invulnerableparticles)))
  (if (> (`self.ChargeTimer`) 0.01)
    (`ActorComponent.Activate` _fireparticles false)
    (else
      (`ActorComponent.Deactivate` _fireparticles))))

(fn `UserConstructionScript`)
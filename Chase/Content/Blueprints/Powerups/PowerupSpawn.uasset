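; Server-side powerup spawn point that periodically spawns a random powerup at its billboard's location during a chase match.
; When the ChaseGameState changes to Playing, it rolls a short random initial delay.
; While Playing, Tick counts that delay down, spawns a random class from PowerupClasses, then rolls a longer random delay for the next spawn.
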(event `GameStateChanged`
  (if (`|EnumEquality` (`ChaseGameState.CurrentGameState` (stale `self.ReceiveBeginPlay` _aschase_game_state)) "Playing")
    (set `self.NextSpawn` (`KismetMathLibrary.RandomFloatInRange` 10.0 40.0))))

(event `self.ReceiveBeginPlay`
  (`/Engine/EditorBlueprintResources/ActorMacros.Switch Has Authority`
    (:`Authority`
      (bind _aschase_game_state (cast `ChaseGameState` (`GameplayStatics.GetGameState`)))
      (add `ChaseGameState.OnGameStateChanged` _aschase_game_state (delegate `GameStateChanged`)))))

(event `self.ReceiveTick`
  (params (DeltaSeconds :type "Float (single-precision)"))
  (bind _nextspawn (`self.NextSpawn`))
  (bind _powerupclasses (`self.PowerupClasses`))
  (`/Engine/EditorBlueprintResources/ActorMacros.Switch Has Authority`
    (:`Authority`
      (bind _aschase_game_state (cast `ChaseGameState` (`GameplayStatics.GetGameState`)))
      (if (`|EnumEquality` (`ChaseGameState.CurrentGameState` _aschase_game_state) "Playing")
        (set `self.NextSpawn` (- _nextspawn DeltaSeconds))
        (if (<= _nextspawn 0.0)
          (set `self.NextSpawn` (`KismetMathLibrary.RandomFloatInRange` 40.0 150.0))
          (`|SpawnActorFromClass` (`KismetArrayLibrary.Array_Get` _powerupclasses (`KismetMathLibrary.RandomIntegerInRange` 0 (- (`KismetArrayLibrary.Array_Length` _powerupclasses) 1))) (`SceneComponent.K2_GetComponentToWorld` (`self.Billboard`))))))))

(fn `UserConstructionScript`)